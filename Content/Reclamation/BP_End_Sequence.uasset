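; BP_End_Sequence is a level actor that plays the game's ending when the wolf player character walks into its trigger volumes.
; It finds the BP_ALS_Wolf instance on BeginPlay and responds only to that actor.
; Overlapping TriggerText reveals the Act2 component.
; Overlapping TriggerCameraFade fades the camera out and holds it, then quits the game after a short delay.
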(event OnComponentBeginOverlap(TriggerCameraFade)
  (params (OverlappedComponent :type Primitive%20Component%20Object%20Reference) (OtherActor :type Actor%20Object%20Reference) (OtherComp :type Primitive%20Component%20Object%20Reference) (OtherBodyIndex :type Integer) (bFromSweep :type Boolean) (SweepResult :type Hit%20Result%20Structure%20%28by%20ref%29))
  (if (== OtherActor (Variables|Default|GetAs%20Syn))
    (CameraFades|StartCameraFade :self (Game|GetPlayerCameraManager 0) :FromAlpha 0.0 :ToAlpha 1.0 :Duration 2.5 :bHoldWhenFinished true)
    (Utilities|FlowControl|Delay 3.0)
    (Game|QuitGame 0 "Quit" false)))

(event OnComponentBeginOverlap(TriggerText)
  (params (OverlappedComponent :type Primitive%20Component%20Object%20Reference) (OtherActor :type Actor%20Object%20Reference) (OtherComp :type Primitive%20Component%20Object%20Reference) (OtherBodyIndex :type Integer) (bFromSweep :type Boolean) (SweepResult :type Hit%20Result%20Structure%20%28by%20ref%29))
  (if (== OtherActor (Variables|Default|GetAs%20Syn))
    (Rendering|SetVisibility (Variables|Default|GetAct%202) true false)))

(event EventBeginPlay
  (bind _returnvalue (Actor|GetActorOfClass "/Game/Reclamation/Core/BP_ALS_Wolf.BP_ALS_Wolf_C"))
  (Variables|Default|SetAs%20Syn _returnvalue))

(fn ConstructionScript)