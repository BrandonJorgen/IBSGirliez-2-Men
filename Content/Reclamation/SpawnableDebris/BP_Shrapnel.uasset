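; BP_Shrapnel is a spawnable debris actor that gets launched by an impulse, shrinks and removes itself.
; Explode applies the supplied impulse to the Shrapnel component, scaled by its mass.
; Tick counts TimeAlive down and lerps the component's relative scale toward zero against a hardcoded five-second span, destroying the actor when the timer runs out.
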(event EventTick
  (params (DeltaSeconds :type Float%20%28single-precision%29))
  (bind _output_get (Variables|Default|SetTimeAlive (- (Variables|Default|GetTimeAlive) DeltaSeconds)))
  (Transformation|SetRelativeScale3D (Variables|Default|GetShrapnel) (Math|Vector|Lerp(Vector) "1.000000,1.000000,1.000000" "0, 0, 0" (- 1.0 (/ _output_get 5.0))))
  (if (<= (Variables|Default|GetTimeAlive) 0.0)
    (Actor|DestroyActor)))

(fn ConstructionScript)

(fn Explode
  (params (Impulse :type Vector))
  (Physics|AddImpulse (Variables|Default|GetShrapnel) Impulse "None" false))